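; Game mode for a shooting game that tracks the current score and a persistent best score.
; On BeginPlay it adds the WBP_Score widget, hides the cursor, sets game-only input and loads the best score.
; AddScore accumulates points and, on a new record, saves it through a BP_SaveGame object to the ScoreData slot.
; Loading falls back to zero when the save is missing or the cast fails.
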(event `self.ReceiveBeginPlay`
  (bind _returnvalue (`GameplayStatics.GetPlayerController` 0))
  ;[1 1 1] 마우스 커서를 숨기고 싶다. 입력을 게임 창에서 받고 싶다.
  (bind _returnvalue_2 (`|CreateWidget` "/Game/Blueprint/WBP_Score.WBP_Score_C"))
  (`UserWidget.AddToViewport` _returnvalue_2 0)
  (set `PlayerController.bShowMouseCursor` false _returnvalue)
  (`WidgetBlueprintLibrary.SetInputMode_GameOnly` _returnvalue)
  (`self.LoadBestScore`))

(event `self.ReceiveTick`
  (params (DeltaSeconds :type "Float (single-precision)")))

(fn `AddScore`
  (params (Value :type Integer))
  ;[1 1 1] Score에 Value(점수)를 누적하고 싶다.
  (bind _output_get (set `self.Score` (+ Value (`self.Score`))))
  ;[1 1 1] 만약 Score가 BestScore보다 크다면 BestScore에 Score값을 대입하고 싶다.
  (if (> _output_get (`self.BestScore`))
    (set `self.BestScore` (`self.Score`))
    (`self.SaveBestScore`)))

(fn `LoadBestScore`
  (bind _returnvalue (`GameplayStatics.DoesSaveGameExist` (`self.ScoreData`)))
  (if _returnvalue
    (bind _returnvalue_2 (`GameplayStatics.LoadGameFromSlot` (`self.ScoreData`)))
    (bind _asbp_save_game (cast `/Game/Blueprint/BP_SaveGame` _returnvalue_2)
      (:`then`
        (set `self.BestScore` (`/Game/Blueprint/BP_SaveGame.SaveBestScore` _asbp_save_game)))
      (:`CastFailed`
        (set `self.BestScore` 0 :!label _label)))
    (else
      (goto _label))))

(fn `SaveBestScore`
  ;[1 1 1] 1, 2, 3 경우의 수를 하고 싶으면 Sequence를 쓸 것! (s누르고 클릭)
  (`|ExecutionSequence`
    (:`then_0`
      ;;[1 1 1] 1. Save Game이라는 클래스를 만든다.
      (bind _returnvalue (`GameplayStatics.CreateSaveGameObject` "/Game/Blueprint/BP_SaveGame.BP_SaveGame_C"))
      (set `self.SaveGameInstance` _returnvalue))
    (:`then_1`
      ;;[1 1 1] 2. 저장한다는 것은 SaveGame 객체를 만들고, 객체의 속성에 저장할 값을 대입한다.
      (set `/Game/Blueprint/BP_SaveGame.SaveBestScore` (`self.BestScore`) (`self.SaveGameInstance`)))
    (:`then_2`
      ;;[1 1 1] 3. 그것을 슬롯(파일)에 저장하는 것이다.
      (`GameplayStatics.SaveGameToSlot` (`self.SaveGameInstance`) (`self.ScoreData`)))))

(fn `UserConstructionScript`)